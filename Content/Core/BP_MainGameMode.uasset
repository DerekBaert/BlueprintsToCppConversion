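; BP_MainGameMode is the main game mode, which sets up the primary on-screen display and owns the quest manager.
; On BeginPlay it creates WBP_MainDisplay for the first player controller, passes in the quest manager, and adds the widget to the viewport.
; GetQuestManager lazily spawns a BP_QuestManager actor on first use and caches it for later calls.
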(event EventBeginPlay
  (bind _returnvalue (UserInterface|CreateWidget "/Game/UI/WBP_MainDisplay.WBP_MainDisplay_C" (Game|GetPlayerController 0) (CallFunction|GetQuestManager)))
  (UserInterface|Viewport|AddtoViewport _returnvalue 0))

(event EventTick
  (params (DeltaSeconds :type Float%20%28single-precision%29)))

(fn ConstructionScript)

(fn GetQuestManager
  (Utilities|IsValid (Variables|Default|GetQuestManager)
    (:Is%20Valid
      (return (Variables|Default|GetQuestManager)))
    (:Is%20Not%20Valid
      (bind _returnvalue (Game|SpawnActorfromClass "/Game/Quests/BP_QuestManager.BP_QuestManager_C" (Math|Transform|MakeTransform "0, 0, 0" "0, 0, 0" "1.000000,1.000000,1.000000") "Undefined" 0 0))
      (bind _output_get (Variables|Default|SetQuestManager _returnvalue))
      (return _output_get))))